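; BP_Spawner randomly populates the level with pickups when play begins.
; It gathers every TargetPoint actor tagged "Spawnpoint" and gives each one a random true/false roll.
; On success, it spawns an actor at that point's transform, using the class of a randomly chosen entry in the Pickups array.
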(event EventBeginPlay
  (bind _pickups (Variables|Default|GetPickups))
  (bind _outactors (Actor|GetAllActorsOfClasswithTag "/Script/Engine.TargetPoint" "Spawnpoint"))
  (for _array_element _outactors
    (bind _result (Math|Integer|DecrementInt (Utilities|Array|Length _pickups))
      (:%20%20
        (if (Math|Random|RandomBool)
          (Game|SpawnActorfromClass (Utilities|GetClass (Utilities|Array|Get(acopy) _pickups (Math|Random|RandomIntegerinRange 0 _result))) (Transformation|GetActorTransform _array_element) "Undefined" "MultiplyWithRoot" 0 0))))))

(fn ConstructionScript)